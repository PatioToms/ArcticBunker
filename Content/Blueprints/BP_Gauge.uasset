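; BP_Gauge is a gauge whose handle rotates between a minimum and maximum rotation to show a value as a fraction of a total.
; SetUpGauge stores the total and snaps the handle to the starting value.
; UpdateGauge clamps each new amount, then a timeline eases the handle from its stored rotation to the target, saving that target on finish.
; AskForActivation always returns false, so activation requests are refused.
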(event `/Game/Blueprints/InteractiveInterface.UpdateGauge`
  (params (CurrentAmount :type Integer))
  (bind _totalvalue (`self.TotalValue`))
  (bind _output_get (set `self.CurrentValue` (`KismetMathLibrary.Conv_IntToDouble` CurrentAmount)))
  (set `self.TargetRotation` (`KismetMathLibrary.RLerp` (`self.MinRotation`) (`self.MaxRotation`) (/ (`KismetMathLibrary.FClamp` _output_get 0.0 _totalvalue) _totalvalue)))
  (bind (_direction _lerp) (`Timeline|GaugeHandleMovement` :!via `PlayFromStart`)
    (:`Update`
      (`SceneComponent.K2_SetRelativeRotation` (`self.Handle`) (`KismetMathLibrary.RLerp` (`self.CurrentRotation`) (`self.TargetRotation`) _lerp) false false))
    (:`Finished`
      (set `self.CurrentRotation` (`self.TargetRotation`)))))

(event `/Game/Blueprints/InteractiveInterface.SetUpGauge`
  (params (TotalValue :type Integer) (CurrentValue :type Integer))
  (set `self.TotalValue` (`KismetMathLibrary.Conv_IntToDouble` TotalValue))
  (bind _output_get (set `self.CurrentValue` (`KismetMathLibrary.Conv_IntToDouble` CurrentValue)))
  (bind _output_get_2 (set `self.CurrentRotation` (`KismetMathLibrary.RLerp` (`self.MinRotation`) (`self.MaxRotation`) (/ _output_get (`self.TotalValue`)))))
  (`SceneComponent.K2_SetRelativeRotation` (`self.Handle`) _output_get_2 false false))

(fn `AskForActivation`
  (params (Item :type "/Game/Blueprints/Data/ItemType Enum" :default "NewEnumerator0") (RequestingSlot :type "/Game/Blueprints/BP_ButtonToggle Object Reference"))
  (returns (CanActivate :type Boolean))
  (return false))

(fn `UserConstructionScript`)