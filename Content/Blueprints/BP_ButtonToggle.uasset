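; Two-sided toggle button that represents an item slot, asking its ParentItem for permission to activate and notifying it on deselect.
; Toggle state drives an Emissive timeline on the displayed material, and disabling an active button switches it off.
; UpdateButtonIcon puts the new icon on the hidden face, sets enabled state from the item type, then flips the mesh 180 degrees after a delay, updating name text and displayed material.
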(event `DisableButton`
  ;[1 1 1] Toggle Button Active
  (if (and (`self.IsEnabled`) (`self.IsToggledActive`))
    (`|ExecutionSequence` :!label _label
      (:`then_0`
        (set `self.IsToggledActive` false))
      (:`then_1`
        (bind (_direction _emissive) (`Timeline|ToggleTimeline` :!via `ReverseFromEnd` :!label _label_2)
          (:`Update`
            (`MaterialInstanceDynamic.SetScalarParameterValue` (`self.DisplayedMaterial`) "Emissive" _emissive)))))))

(event `self.DoSomething`
  (bind _parentitem (`self.ParentItem`))
  ;[1 1 1] Toggle Button Active
  (if (`self.IsToggledActive`)
    (message `/Game/Blueprints/InteractiveInterface.DeSelectItem` (`self.ParentItem`))
    (goto _label)
    (elif (and (`KismetSystemLibrary.IsValid` _parentitem) (`|EnumInequality` (`self.CurrentlyContainedItem`) "NewEnumerator5"))
      (bind _canactivate (message `/Game/Blueprints/InteractiveInterface.AskForActivation` _parentitem (`self.CurrentlyContainedItem`) self))
      (if _canactivate
        (`|ExecutionSequence`
          (:`then_0`
            (goto _label_2 :!via `PlayFromStart`))
          (:`then_1`
            (set `self.IsToggledActive` true)))))))

(event `UpdateButtonIcon`
  (params (NewMaterial :type "MaterialInstance Object Reference") (NewItem :type "/Game/Blueprints/Data/ItemType Enum" :default "NewEnumerator0") (NewName :type Text :default "NSLOCTEXT(\"[00DE494B40EBBBD311394EBF904F20D7]\", \"A2D7A61246EE29D4F1F135BFBA8F5514\", \"Erg\")"))
  ;[1 1 1] Change Button Icon
  (if (`self.IsBackwards`)
    (bind _returnvalue (`PrimitiveComponent.CreateDynamicMaterialInstance` (`self.ButtonMesh`) 1 NewMaterial "FrontMaterial"))
    (set `self.BackMaterial` _returnvalue)
    (else
      (bind _returnvalue_2 (`PrimitiveComponent.CreateDynamicMaterialInstance` (`self.ButtonMesh`) 2 NewMaterial "BackMaterial"))
      (set `self.FrontMaterial` _returnvalue_2)))
  ;;[1 1 1] ButtonActivation
  (bind _output_get (set `self.CurrentlyContainedItem` NewItem))
  (if (and (`self.IsEnabled`) (`|EnumEquality` _output_get "NewEnumerator5"))
    (`self.SetEnabled` false)
    (else
      (`self.SetEnabled` true)))
  (`KismetSystemLibrary.Delay` 0.6)
  (if (not (`self.IsBackwards`))
    (bind (_direction _lerptrack) (`Timeline|ButtonFlipTimeline` :!via `PlayFromStart` :!label _label_3)
      (:`Update`
        (`SceneComponent.K2_SetRelativeRotation` (`self.ButtonMesh`) (`KismetMathLibrary.RLerp` (struct) (struct :`Roll` 180.0) _lerptrack) false false))
      (:`Finished`
        (`TextRenderComponent.K2_SetText` (`self.Item Name`) NewName)
        (bind _output_get_2 (set `self.IsBackwards` (not (`self.IsBackwards`))))
        (if _output_get_2
          (set `self.DisplayedMaterial` (`self.FrontMaterial`))
          (else
            (set `self.DisplayedMaterial` (`self.BackMaterial`))))))
    (else
      (goto _label_3 :!via `ReverseFromEnd`))))

(fn `UserConstructionScript`
  (bind _buttonmesh (`self.ButtonMesh`))
  (`parent.UserConstructionScript`)
  (bind _returnvalue (`PrimitiveComponent.CreateDynamicMaterialInstance` _buttonmesh 1 (`PrimitiveComponent.GetMaterial` _buttonmesh 1) "None"))
  (bind _output_get (set `self.FrontMaterial` _returnvalue))
  (set `self.DisplayedMaterial` _output_get))