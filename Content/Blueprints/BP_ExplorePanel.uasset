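; Two-sided in-world panel for choosing where to explore (Storage, Forest or Campfire), with action point and frostbite costs shown as lit bulbs.
; The construction script builds the bulb rows; their emissive parameters follow each location's costs, including frostbite penalty on AP.
; Timelines slide the frame and flip the panel, updating the hidden face before it shows.
; Confirming asks the parent actor to check AP, then hides the panel, applies effects and explores.
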(event Custom|RevealPanel
  ;[1 0.1607 0] Reveal and Hide Panel
  (Utilities|FlowControl|Sequence
    (:then_0
      (Variables|/Game/Blueprints/BP_ButtonParent.BP_ButtonParent_C|SetIsEnabled (Variables|InterfaceActors|GetBackButton) true)
      (CallFunction|InitialCheck)
      (CallFunction|ResetSelection)
      (bind _distancelerp (Timeline|EventTravelTimeline Play)
        (:Update
          (Transformation|SetWorldLocation (Variables|Default|GetEventFrame) (Math|Vector|Lerp(Vector) (Variables|Default|GetCurrentLocation) (Variables|Default|GetTargetLocation) _distancelerp) false false))))
    (:then_1
      (Utilities|FlowControl|DoOnce true) ; enters at Reset
    )))

(event Custom|HidePanel
  ;[1 0.1607 0] Reveal and Hide Panel
  (Utilities|FlowControl|DoOnce true
    (:Completed
      (Variables|/Game/Blueprints/BP_GameCoordinator.BP_GameCoordinator_C|SetIsBusy (Variables|Default|GetParentActor) false)
      (Variables|/Game/Blueprints/BP_ButtonParent.BP_ButtonParent_C|SetIsEnabled (Variables|InterfaceActors|GetBackButton) false)
      (bind _distancelerp (Timeline|EventTravelTimeline Reverse)
        (:Update
          (Transformation|SetWorldLocation (Variables|Default|GetEventFrame) (Math|Vector|Lerp(Vector) (Variables|Default|GetCurrentLocation) (Variables|Default|GetTargetLocation) _distancelerp) false false))))))

(event Custom|NextOption
  (bind _okbuttona (Variables|InterfaceActors|GetOkButtonA))
  (bind _okbuttonb (Variables|InterfaceActors|GetOkButtonB))
  ;[1 0.1607 0] Location Panel Switching
  (Utilities|FlowControl|DoOnce false
    (:Completed
      (Utilities|FlowControl|Sequence
        (:then_0
          ;;[1 1 1] Flip the event panel
          (bind _output_get (Variables|Default|SetCurrentRotation (Transformation|GetWorldRotation (Variables|Default|GetLocationPanel))))
          (Variables|Default|SetTargetRotation (Math|Rotator|MakeRotator (.roll _output_get) (+ (.pitch _output_get) 180.100006) (.yaw _output_get)))
          (bind _lerptrack (Timeline|PanelRotationTimeline PlayFromStart)
            (:Update
              (Transformation|SetRelativeRotation (Variables|Default|GetLocationPanel) (Math|Rotator|Lerp(Rotator) (Variables|Default|GetCurrentRotation) (Variables|Default|GetTargetRotation) _lerptrack true) false false))
            (:Finished
              (Variables|Default|SetIsFaceAInFront (not (Variables|Default|GetIsFaceAInFront)))
              (CallFunction|OptionCooldown))))
        (:then_1
          ;;[1 1 1] Set Material and Buttons on the opposite side
          (Math|Integer|IncrementInt (Variables|Default|GetCurrentSelectionInt)
            (:%20%20
              (bind (_nextmaterial _ap _frostbite) (CallFunction|SelectLocation))
              (if (Variables|Default|GetIsFaceAInFront)
                (CallFunction|UpdateLightStates (Variables|Default|GetAPMeshesSideB) _ap)
                (CallFunction|UpdateLightStates (Variables|Default|GetFrostbiteMeshesSideB) _frostbite)
                (Rendering|Material|SetMaterial (Variables|Default|GetLocationPanel) 2 _nextmaterial)
                (Variables|/Game/Blueprints/BP_ButtonParent.BP_ButtonParent_C|SetIsEnabled _okbuttona false)
                (Variables|/Game/Blueprints/BP_ButtonParent.BP_ButtonParent_C|SetIsEnabled _okbuttonb true)
                (else
                  (CallFunction|UpdateLightStates (Variables|Default|GetAPMeshesSideA) _ap)
                  (CallFunction|UpdateLightStates (Variables|Default|GetFrostbiteMeshesSideA) _frostbite)
                  (Rendering|Material|SetMaterial (Variables|Default|GetLocationPanel) 1 _nextmaterial)
                  (Variables|/Game/Blueprints/BP_ButtonParent.BP_ButtonParent_C|SetIsEnabled _okbuttona true)
                  (Variables|/Game/Blueprints/BP_ButtonParent.BP_ButtonParent_C|SetIsEnabled _okbuttonb false))))))))))

(event Custom|OptionCooldown
  (bind _okbuttona (Variables|InterfaceActors|GetOkButtonA))
  (bind _okbuttonb (Variables|InterfaceActors|GetOkButtonB))
  ;[1 0.1607 0] Location Panel Switching
  (Utilities|FlowControl|DoOnce false) ; enters at Reset
)

(event Custom|ConfirmSelection
  (bind _currentselectionenum (Variables|Default|GetCurrentSelectionEnum))
  (bind _parentactor (Variables|Default|GetParentActor))
  ;[1 0.1607 0] Ask Game Coordinator if we can Explore
  (Utilities|FlowControl|DoOnce true
    (:Completed
      (bind _canexplore (Default|LocationAPCostCheck _parentactor (Variables|Default|GetCurrentSelectionEnum)))
      (if _canexplore
        (CallFunction|HidePanel)
        (Utilities|FlowControl|Delay 0.5)
        (bind (_cancontinue _delay) (Default|ApplyExploreEffects _parentactor _currentselectionenum))
        (if _cancontinue
          (Utilities|FlowControl|Delay _delay)
          (Default|Explore _parentactor _currentselectionenum))
        (else
          (CallFunction|ResetSelection))))))

(event Custom|ResetSelection
  (bind _currentselectionenum (Variables|Default|GetCurrentSelectionEnum))
  (bind _parentactor (Variables|Default|GetParentActor))
  ;[1 0.1607 0] Ask Game Coordinator if we can Explore
  (Utilities|FlowControl|DoOnce true) ; enters at Reset
)

(event Custom|InitialCheck
  ;[1 0.1607 0] Update Front Panel
  (bind (_nextmaterial _ap _frostbite) (CallFunction|SelectLocation))
  (if (not (Variables|Default|GetIsFaceAInFront))
    (CallFunction|UpdateLightStates (Variables|Default|GetAPMeshesSideB) _ap)
    (CallFunction|UpdateLightStates (Variables|Default|GetFrostbiteMeshesSideB) _frostbite)
    (else
      (CallFunction|UpdateLightStates (Variables|Default|GetAPMeshesSideA) _ap)
      (CallFunction|UpdateLightStates (Variables|Default|GetFrostbiteMeshesSideA) _frostbite))))

(event EventBeginPlay
  (bind _backbutton (Variables|InterfaceActors|GetBackButton))
  (bind _nextbutton (Variables|InterfaceActors|GetNextButton))
  (bind _okbuttona (Variables|InterfaceActors|GetOkButtonA))
  (bind _okbuttonb (Variables|InterfaceActors|GetOkButtonB))
  ;[0 1 0.9768] Assign Buttons
  (Utilities|FlowControl|Sequence
    (:then_0
      (Utilities|IsValid _backbutton
        (:Is%20Valid
          (EventDispatchers|BindEventtoButtonIsTriggered _backbutton (EventDispatchers|CreateEvent :!event Custom|HidePanel)))))
    (:then_1
      (Utilities|IsValid _nextbutton
        (:Is%20Valid
          (EventDispatchers|BindEventtoButtonIsTriggered _nextbutton (EventDispatchers|CreateEvent :!event Custom|NextOption)))))
    (:then_2
      (Utilities|IsValid _okbuttona
        (:Is%20Valid
          (EventDispatchers|BindEventtoButtonIsTriggered _okbuttona (EventDispatchers|CreateEvent :!event Custom|ConfirmSelection))
          (Transformation|AttachComponentToComponent _okbuttona (Variables|Default|GetButtonPivotFaceA) "None" "SnapToTarget" "SnapToTarget" "KeepWorld" false))))
    (:then_3
      (Utilities|IsValid _okbuttonb
        (:Is%20Valid
          (EventDispatchers|BindEventtoButtonIsTriggered _okbuttonb (EventDispatchers|CreateEvent :!event Custom|ConfirmSelection))
          (Transformation|AttachComponentToComponent _okbuttonb (Variables|Default|GetButtonPivotFaceB) "None" "SnapToTarget" "SnapToTarget" "KeepWorld" false))))))

(fn ConstructionScript
  (bind _output_get (Variables|Default|SetCurrentLocation (Transformation|GetWorldLocation (Variables|Default|GetEventFrame))))
  (Variables|Default|SetTargetLocation (Math|Vector|MakeVector (.x _output_get) (.y _output_get) (- (.z _output_get) (Variables|Default|GetTravelDistance))))
  (Utilities|FlowControl|Sequence
    (:then_0
      (bind _resultingmesharray (CallFunction|SetUpLightbulbArray "/Game/Materials/MI_GenericEmissive.MI_GenericEmissive" (Variables|Default|GetButtonPivotFaceA) (Variables|Default|GetAPMeshesSideA) (Variables|Default|GetMaxActionPoints) (* (Variables|Default|GetLightbulbCenterOffset) -1.0) (Variables|Default|GetLightbulbSeparation) 63.0 -6.0 2e+01))
      (Variables|Default|SetAPMeshesSideA _resultingmesharray)
      (bind _resultingmesharray_2 (CallFunction|SetUpLightbulbArray "/Game/Materials/MI_GenericEmissive.MI_GenericEmissive" (Variables|Default|GetButtonPivotFaceB) (Variables|Default|GetAPMeshesSideB) (Variables|Default|GetMaxActionPoints) (Variables|Default|GetLightbulbCenterOffset) (Variables|Default|GetLightbulbSeparation) -63.0 6.0 4e+01))
      (Variables|Default|SetAPMeshesSideB _resultingmesharray_2))
    (:then_1
      (bind _resultingmesharray_3 (CallFunction|SetUpLightbulbArray "/Game/Materials/MI_FrostbiteMat.MI_FrostbiteMat" (Variables|Default|GetButtonPivotFaceA) (Variables|Default|GetFrostbiteMeshesSideA) (Variables|Default|GetMaxFrostbite) (Variables|Default|GetLightbulbCenterOffset) (Variables|Default|GetLightbulbSeparation) 63.0 6.0 2e+01))
      (Variables|Default|SetFrostbiteMeshesSideA _resultingmesharray_3)
      (bind _resultingmesharray_4 (CallFunction|SetUpLightbulbArray "/Game/Materials/MI_FrostbiteMat.MI_FrostbiteMat" (Variables|Default|GetButtonPivotFaceB) (Variables|Default|GetFrostbiteMeshesSideB) (Variables|Default|GetMaxFrostbite) (* (Variables|Default|GetLightbulbCenterOffset) -1.0) (Variables|Default|GetLightbulbSeparation) -63.0 -6.0 4e+01))
      (Variables|Default|SetFrostbiteMeshesSideB _resultingmesharray_4))))

(fn SelectLocation
  (bind _locationcosts (Variables|Default|GetLocationCosts))
  (bind _locationcosts_2 (Variables|Default|GetLocationCosts))
  (bind _locationcosts_3 (Variables|Default|GetLocationCosts))
  (bind (_frostbiteperturn _campapcost _campfrostbitecost) (Utilities|Struct|BreakBlizzardStruct _locationcosts))
  (bind (_frostbiteperturn_2 _campapcost_2 _campfrostbitecost_2 _storageapcost _storagefrostbitecost) (Utilities|Struct|BreakBlizzardStruct _locationcosts_2))
  (bind (_frostbiteperturn_3 _campapcost_3 _campfrostbitecost_3 _storageapcost_2 _storagefrostbitecost_2 _forestapcost _forestfrostbitecost) (Utilities|Struct|BreakBlizzardStruct _locationcosts_3))
  (if (> (Variables|Default|GetCurrentSelectionInt) 3)
    (Variables|Default|SetCurrentSelectionInt 1))
  (switch int (Variables|Default|GetCurrentSelectionInt)
    (:1
      (Variables|Default|SetCurrentSelectionEnum "NewEnumerator0")
      (return "/Game/Materials/MI_LocationPanel_Storage.MI_LocationPanel_Storage" (+ (Variables|Default|GetFrostbitePenalty) _storageapcost) _storagefrostbitecost))
    (:2
      (Variables|Default|SetCurrentSelectionEnum "NewEnumerator1")
      (return "/Game/Materials/MI_LocationPanel_Forest.MI_LocationPanel_Forest" (+ (Variables|Default|GetFrostbitePenalty) _forestapcost) _forestfrostbitecost))
    (:3
      (Variables|Default|SetCurrentSelectionEnum "NewEnumerator2")
      (return "/Game/Materials/MI_LocationPanel_Campfire.MI_LocationPanel_Campfire" (+ (Variables|Default|GetFrostbitePenalty) _campapcost) _campfrostbitecost))))

(fn SetUpLightbulbArray
  (params (TargetMaterial :type Material%20Instance%20Object%20Reference) (ReferencePoint :type Scene%20Component%20Object%20Reference) (ArrayToOverride :type Array%20of%20Static%20Mesh%20Component%20Object%20References) (NumberOfLighbulbs :type Integer) (OffsetFromCenter :type Float%20%28single-precision%29) (SeparationBetweenLightBulbs :type Float%20%28single-precision%29) (XDistance :type Float%20%28single-precision%29) (DistributionRadius :type Float%20%28single-precision%29) (ZOffset :type Float%20%28single-precision%29))
  (LocalVariables|SetLightbulbMaterial TargetMaterial)
  (LocalVariables|SetRefPoint ReferencePoint)
  (bind _output_get (LocalVariables|SetMainArray ArrayToOverride))
  (if (> (Utilities|Array|Length _output_get) 0)
    (for _array_element _output_get
      (Components|DestroyComponent _array_element))
    (Utilities|Array|Clear (LocalVariables|GetMainArray)))
  (for _index (range 0 (- NumberOfLighbulbs 1))
    (bind _returnvalue (AddComponent|AddStaticMeshComponent false (Math|Transform|MakeTransform (Math|Vector|MakeVector (+ (.z (Variables|/Script/Engine.SceneComponent|GetRelativeLocation (LocalVariables|GetRefPoint))) XDistance) (|(X+(((Sin(A))*B)+C)) _index DistributionRadius OffsetFromCenter (.y (Variables|/Script/Engine.SceneComponent|GetRelativeLocation (LocalVariables|GetRefPoint)))) (|(X+(C-(A*B))) (.x (Variables|/Script/Engine.SceneComponent|GetRelativeLocation (LocalVariables|GetRefPoint))) _index SeparationBetweenLightBulbs (Math|Float|MakeLiteralFloat ZOffset))) "0.000000, 0,90.000000" "0.050000,0.050000,0.050000")))
    (Utilities|Array|Add (LocalVariables|GetMainArray) _returnvalue))
  (for _array_element_2 (LocalVariables|GetMainArray)
    (Utilities|FlowControl|Sequence
      (:then_0
        (Components|StaticMesh|SetStaticMesh _array_element_2 "/Game/Meshes/SM_GaugeGlass.SM_GaugeGlass"))
      (:then_1
        (Rendering|Material|SetMaterial _array_element_2 0 (LocalVariables|GetLightbulbMaterial)))
      (:then_2
        (Transformation|AttachComponentToComponent _array_element_2 (LocalVariables|GetRefPoint) "None" "KeepWorld" "KeepWorld" "KeepWorld" true))))
  (return (LocalVariables|GetMainArray)))

(fn UpdateLightStates
  (params (MeshArrayToChange :type Array%20of%20Static%20Mesh%20Component%20Object%20References) (LitLightBulbs :type Integer))
  (for (_array_element _array_index) MeshArrayToChange
    (if (> _array_index (- (Math|Integer|Absolute(Integer) LitLightBulbs) 1))
      (Rendering|Material|SetScalarParameterValueonMaterials _array_element "Emissive" 0.0)
      (else
        (Rendering|Material|SetScalarParameterValueonMaterials _array_element "Emissive" 15.0)))))

(fn AskforActivation
  (params (Item :type ItemType%20Enum :default "NewEnumerator0") (RequestingSlot :type BP%20Button%20Toggle%20Object%20Reference))
  (return false))