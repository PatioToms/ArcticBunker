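; BP_ActionButton is a button that passes its assigned action (Use, Burn, Store or Refine) to its parent BP_GameCoordinator and displays an AP cost.
; The construction script sets the icon, starting flip state and a centred row of lightbulb meshes sized by max AP cost.
; UpdateAPCost lights bulbs to match the cost, and ErrorFeedback animates their emissive material.
; Reveal and hide flip the plaque through a randomly delayed timeline, toggling its enabled state.
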(event Custom|HidePanel
  (if (not (Variables|Default|GetIsHidden))
    (Utilities|FlowControl|Delay (Math|Random|RandomFloatinRange 0.0 0.3))
    (bind _lerptrack (Timeline|PlaqueFlipTimeline ReverseFromEnd)
      (:Update
        (Transformation|SetWorldRotation (Variables|Default|GetButtonBaseMesh) (Math|Rotator|Lerp(Rotator) "-90.000000,0.000000, 0" "90.000000,0.000000, 0" _lerptrack) false false))
      (:Finished
        (bind _output_get (Variables|Default|SetIsHidden (not (Variables|Default|GetIsHidden))))
        (Variables|Default|SetIsEnabled (not _output_get))))))

(event Custom|RevealPanel
  (if (Variables|Default|GetIsHidden)
    (Utilities|FlowControl|Delay (Math|Random|RandomFloatinRange 0.0 0.3))
    (bind _lerptrack (Timeline|PlaqueFlipTimeline PlayFromStart)
      (:Update
        (Transformation|SetWorldRotation (Variables|Default|GetButtonBaseMesh) (Math|Rotator|Lerp(Rotator) "-90.000000,0.000000, 0" "90.000000,0.000000, 0" _lerptrack) false false))
      (:Finished
        (bind _output_get (Variables|Default|SetIsHidden (not (Variables|Default|GetIsHidden))))
        (Variables|Default|SetIsEnabled (not _output_get))))))

(event EventErrorFeedback
  (bind _erroremissivetrack (Timeline|ErrorFeedbackTimeline PlayFromStart)
    (:Update
      (Rendering|Material|SetScalarParameterValueonMaterials (Variables|Default|GetIlluminatedArray) "ErrorLerp" _erroremissivetrack))))

(event EventDoSomething
  (bind _asbp_game_coordinator (Utilities|Casting|CastToBP_GameCoordinator (Variables|Default|GetParentItem)))
  (Default|ApplyAction _asbp_game_coordinator (Variables|Default|GetAssignedAction)))

(fn ConstructionScript
  (bind _buttonbasemesh (Variables|Default|GetButtonBaseMesh))
  (bind _maxapcost (Variables|Default|GetMaxAPCost))
  (bind _buttonmesh (Variables|Default|GetButtonMesh))
  (|CallParentFunction)
  (Utilities|FlowControl|Sequence
    (:then_0
      ;[1 1 1] Setting Up Button Icon
      (switch Utilities|FlowControl|Switch|SwitchonActionType (Variables|Default|GetAssignedAction)
        (:NewEnumerator0
          (Rendering|Material|SetMaterial _buttonmesh 1 "/Game/Materials/MI_ButtonIcon_Use.MI_ButtonIcon_Use"))
        (:NewEnumerator1
          (Rendering|Material|SetMaterial _buttonmesh 1 "/Game/Materials/MI_ButtonIcon_Burn.MI_ButtonIcon_Burn"))
        (:NewEnumerator4
          (Rendering|Material|SetMaterial _buttonmesh 1 "/Game/Materials/MI_ButtonIcon_Store.MI_ButtonIcon_Store"))
        (:NewEnumerator2
          (Rendering|Material|SetMaterial _buttonmesh 1 "/Game/Materials/MI_ButtonIcon_Refine.MI_ButtonIcon_Refine"))))
    (:then_1
      ;[1 1 1] Setting Up Button Position
      (if (Variables|Default|GetIsEnabled)
        (Transformation|SetWorldRotation _buttonbasemesh "90.000000, 0, 0" false false)
        (Variables|Default|SetIsHidden false)
        (else
          (Transformation|SetWorldRotation _buttonbasemesh "-90.000000, 0, 0" false false)
          (Variables|Default|SetIsHidden true))))
    (:then_2
      (Utilities|Array|Clear (Variables|Default|GetLightBulbArray))
      (for _index (range 0 (- _maxapcost 1))
        (bind _returnvalue (AddComponent|AddStaticMeshComponent false (Math|Transform|MakeTransform (Math|Vector|MakeVector -35.0 (+ (|((CurrentIndex*distance)-((round((TotalIndex/2)))*distance)) _index (Variables|Default|GetLightbulbSeparation) _maxapcost) 1.5e+02) 0.0) "-90.000000,0.000000, 0" "0.100000,0.100000,0.100000")))
        (Utilities|Array|Add (Variables|Default|GetLightBulbArray) _returnvalue)))))

(fn UpdateAPCost
  (params (NewAPCost :type Integer))
  (Utilities|Array|Clear (Variables|Default|GetIlluminatedArray))
  (for (_array_element _array_index) (Variables|Default|GetLightBulbArray)
    (if (> _array_index (- (Math|Integer|Absolute(Integer) NewAPCost) 1))
      (Rendering|Material|SetMaterial _array_element 0 "/Game/Materials/MI_GenericEmissive_OFF.MI_GenericEmissive_OFF")
      (else
        (Rendering|Material|SetMaterial _array_element 0 "/Game/Materials/MI_GenericEmissive.MI_GenericEmissive")
        (Utilities|Array|Add (Variables|Default|GetIlluminatedArray) _array_element)))))