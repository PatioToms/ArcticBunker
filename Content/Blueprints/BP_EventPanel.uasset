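; Event panel actor that slides into view to show an event or obtained item with an OK button.
; Update functions fill the text widget from event or item data tables and store the action, stat and item.
; RevealEvent lowers the frame via timeline and re-arms a DoOnce, which HideEvent fires to reverse it.
; After a short delay, the parent actor applies the stored effect.
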(event `self.ReceiveBeginPlay`
  (bind _asgeneric_text_widget (cast `/Game/Widgets/GenericTextWidget` (`WidgetComponent.GetUserWidgetObject` (`self.EventPanelWidget`))))
  (set `self.TextWidget` _asgeneric_text_widget))

(event `RevealEvent`
  (`|ExecutionSequence`
    (:`then_0`
      (set `/Game/Blueprints/BP_ButtonParent.IsEnabled` true (`self.OkButton`))
      (bind (_direction _distancelerp) (`Timeline|EventTravelTimeline` :!label _label)
        (:`Update`
          (`SceneComponent.K2_SetWorldLocation` (`self.EventFrame`) (`KismetMathLibrary.VLerp` (`self.CurrentLocation`) (`self.TargetLocation`) _distancelerp) false false))))
    (:`then_1`
      (goto _label_2 :!via `Reset`))))

(event `HideEvent`
  (`/Engine/EditorBlueprintResources/StandardMacros.DoOnce` true :!label _label_2
    (:`Completed`
      (`|ExecutionSequence`
        (:`then_0`
          (set `/Game/Blueprints/BP_ButtonParent.IsEnabled` false (`self.OkButton`))
          (goto _label :!via `Reverse`))
        (:`then_1`
          (`KismetSystemLibrary.Delay` 0.5)
          (`/Game/Blueprints/BP_GameCoordinator.ApplyEventEffect` (`self.ParentActor`) (`self.Action`) (`self.Item`) (`self.Stat`)))))))

(fn `AskForActivation`
  (params (Item :type "/Game/Blueprints/Data/ItemType Enum" :default "NewEnumerator0") (RequestingSlot :type "/Game/Blueprints/BP_ButtonToggle Object Reference"))
  (returns (CanActivate :type Boolean))
  (return false))

(fn `UpdateEventPanel`
  (params (EventID :type String))
  (bind _returnvalue (`|GetDataTableRow` "/Game/Blueprints/Data/EventDataTable.EventDataTable" (`KismetStringLibrary.Conv_StringToName` EventID))
    (:`then`
      (bind (_title _description _effect _stateffect _associateditem _associatedmaterial) (break `/Game/Blueprints/Data/EventStruct` _returnvalue))
      (`/Game/Widgets/GenericTextWidget.UpdateEventWidget` (`self.TextWidget`) _title _description (`WidgetBlueprintLibrary.MakeBrushFromTexture` null))
      (set `self.Action` _effect)
      (set `self.Stat` _stateffect)
      (set `self.Item` _associateditem))))

(fn `UpdateItemPanel`
  (params (ObtainedItem :type "/Game/Blueprints/Data/ItemType Enum" :default "NewEnumerator0"))
  (bind _output_get (set `self.Item` ObtainedItem))
  (bind _returnvalue (`|GetDataTableRow` "/Game/Blueprints/Data/ItemDataTable.ItemDataTable" (`KismetStringLibrary.Conv_StringToName` (`|GetEnumeratorNameAsString` _output_get)))
    (:`then`
      (`|ExecutionSequence`
        (:`then_0`
          (set `self.Action` "NewEnumerator1"))
        (:`then_1`
          (bind (_displayname _description _arrayofpossibleactions _inventorybuttonicon _itemtexture) (break `/Game/Blueprints/Data/ItemStruct` _returnvalue))
          (`/Game/Widgets/GenericTextWidget.UpdateEventWidget` (`self.TextWidget`) _displayname _description (`WidgetBlueprintLibrary.MakeBrushFromTexture` _itemtexture 256 256))
          (`WidgetComponent.RequestRedraw` (`self.EventPanelWidget`)))))))

(fn `UserConstructionScript`
  (bind _output_get (set `self.CurrentLocation` (`SceneComponent.K2_GetComponentLocation` (`self.EventFrame`))))
  (set `self.TargetLocation` (`KismetMathLibrary.MakeVector` (.x _output_get) (.y _output_get) (- (.z _output_get) (`self.TravelDistance`))))
  (add `/Game/Blueprints/BP_ButtonParent.ButtonIsTriggered` (`self.OkButton`) (`|CreateDelegate` :!event `HideEvent`)))