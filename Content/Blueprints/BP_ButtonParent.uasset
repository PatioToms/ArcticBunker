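; Base actor for clickable 3D buttons, with empty DoSomething and default-false AskForActivation functions as apparent hooks for children.
; A click on an enabled, unselected button plays a press timeline and, after a short delay, calls DoSomething and a DoOnce-gated ButtonIsTriggered dispatcher.
; Timelines flash error emissive and lower and dim the button when disabled, reversing on re-enable.
; The construction script applies configurable meshes and materials.
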(event `/Game/Blueprints/InteractiveInterface.ErrorFeedback`
  ;[0 1 0.1464] Error Feedback
  (bind (_direction _emissivetrack) (`Timeline|ErrorTimeline` :!via `PlayFromStart`)
    (:`Update`
      (`MeshComponent.SetScalarParameterValueOnMaterials` (`self.ButtonMesh`) "ErrorEmissive" _emissivetrack))))

(event `self.ReceiveActorOnClicked`
  (params (ButtonPressed :type "Key Structure"))
  ;[1 0.1607 0] General Behaviour
  (if (and (not (`self.IsSelected`)) (`self.IsEnabled`))
    (`|ExecutionSequence`
      (:`then_0`
        (bind (_direction _lerp) (`Timeline|ButtonPressTimeline` :!via `PlayFromStart`)
          (:`Update`
            (`SceneComponent.K2_SetRelativeLocation` (`self.ButtonPivot`) (`KismetMathLibrary.VLerp` (0.0 0.0 20.0) (0.0 0.0 2.0) _lerp) false false))
          (:`Finished`
            (set `self.IsSelected` false)
            (goto _label :!via `Reset`))))
      (:`then_1`
        (set `self.IsSelected` true))
      (:`then_2`
        (`KismetSystemLibrary.Delay` 0.2)
        (`self.DoSomething`)
        (`/Engine/EditorBlueprintResources/StandardMacros.DoOnce` false :!label _label
          (:`Completed`
            (`self.ButtonIsTriggered`)))))))

(event `/Game/Blueprints/InteractiveInterface.SetEnabled`
  (params (NewEnabled :type Boolean))
  ;[0 1 0.1464] Enabled / Disabled Behaviour
  (if (!= NewEnabled (`self.IsEnabled`))
    (bind _output_get (set `self.IsEnabled` NewEnabled))
    (if (not _output_get)
      (bind (_direction _lerptrack) (`Timeline|DisabledTimeline` :!via `PlayFromStart` :!label _label_2)
        (:`Update`
          (`SceneComponent.K2_SetRelativeLocation` (`self.ButtonPivot`) (`KismetMathLibrary.VLerp` (0.0 0.0 20.0) (0.0 0.0 8.0) _lerptrack) false false)
          (`MeshComponent.SetScalarParameterValueOnMaterials` (`self.ButtonMesh`) "Emissive" (`KismetMathLibrary.Lerp` 0.5 0.0 _lerptrack))))
      (else
        (goto _label_2 :!via `ReverseFromEnd`)))))

(fn `AskForActivation`
  (params (Item :type "/Game/Blueprints/Data/ItemType Enum" :default "NewEnumerator0") (RequestingSlot :type "/Game/Blueprints/BP_ButtonToggle Object Reference"))
  (returns (CanActivate :type Boolean))
  (return false))

(fn `DoSomething`)

(fn `UserConstructionScript`
  (`|ExecutionSequence`
    (:`then_0`
      (`StaticMeshComponent.SetStaticMesh` (`self.ButtonMesh`) (`self.Button`))
      (`StaticMeshComponent.SetStaticMesh` (`self.ButtonBaseMesh`) (`self.ButtonBase`)))
    (:`then_1`
      (`PrimitiveComponent.SetMaterial` (`self.ButtonMesh`) 2 (`self.ButtonFaceB`))
      (`PrimitiveComponent.SetMaterial` (`self.ButtonMesh`) 1 (`self.ButtonFaceA`))
      (`PrimitiveComponent.SetMaterial` (`self.ButtonMesh`) 0 (`self.ButtonBaseMaterial`))
      (`PrimitiveComponent.SetMaterial` (`self.ButtonBaseMesh`) 0 (`self.ButtonBaseMaterial`)))))