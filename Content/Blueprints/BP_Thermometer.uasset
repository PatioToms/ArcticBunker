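; Thermometer gauge actor that displays an amount by scaling the Z axis of its bar mesh.
; SetUpGauge stores the maximum and snaps the bar to the normalized, clamped starting value, while UpdateGauge animates changes through a timeline lerp.
; Updates arriving mid-animation overwrite a single cached target, which replays when the timeline finishes, so only the latest pending value is shown.
; AskForActivation always returns false.
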(event `/Game/Blueprints/InteractiveInterface.SetUpGauge`
  (params (TotalValue :type Integer) (CurrentValue :type Integer))
  ;[1 1 1] Set Up Gauge
  (bind _output_get (set `self.GaugeMax` (`KismetMathLibrary.Conv_IntToDouble` TotalValue)))
  (bind _output_get_2 (set `self.CurrentValue` (`KismetMathLibrary.FClamp` (`KismetMathLibrary.NormalizeToRange` (`KismetMathLibrary.Conv_IntToDouble` CurrentValue) 0.0 _output_get) 0.01)))
  (`SceneComponent.SetRelativeScale3D` (`self.SM_ThermometerBar`) (`KismetMathLibrary.MakeVector` 1.0 0.75 _output_get_2)))

(event `self.ReceiveBeginPlay`
  (bind (_relativescale3d_x _relativescale3d_y _relativescale3d_z) (`KismetMathLibrary.BreakVector` (`SceneComponent.RelativeScale3D` (`self.SM_ThermometerBar`))))
  ;[1 1 1] Set-Up "current value" variable on Begin Play
  (set `self.CurrentValue` _relativescale3d_z))

(event `RetriggerTimeline`
  (params (CacheValue :type "Float (double-precision)"))
  (bind _cachevalue (`self.CacheValue`))
  ;[1 1 1] Update Gauge
  (set `self.TargetValue` CacheValue)
  (set `self.CacheValue` -1.0)
  (bind (_direction _lerptrack) (`Timeline|InterpTimeline` :!via `PlayFromStart` :!label _label)
    (:`Update`
      (`SceneComponent.SetRelativeScale3D` (`self.SM_ThermometerBar`) (`KismetMathLibrary.MakeVector` 1.0 0.75 (`KismetMathLibrary.Lerp` (`self.CurrentValue`) (`self.TargetValue`) _lerptrack))))
    (:`Finished`
      (set `self.CurrentValue` (`self.TargetValue`))
      (if (!= _cachevalue -1.0)
        (`self.RetriggerTimeline` _cachevalue)))))

(event `/Game/Blueprints/InteractiveInterface.UpdateGauge`
  (params (CurrentAmount :type Integer))
  (bind _returnvalue (`KismetMathLibrary.FClamp` (`KismetMathLibrary.NormalizeToRange` (`KismetMathLibrary.Conv_IntToDouble` CurrentAmount) 0.0 (`self.GaugeMax`)) 0.01))
  ;[1 1 1] Update Gauge
  (if (not (`TimelineComponent.IsPlaying` (`self.InterpTimeline`)))
    (set `self.TargetValue` _returnvalue)
    (goto _label :!via `PlayFromStart`)
    (else
      (set `self.CacheValue` _returnvalue))))

(fn `AskForActivation`
  (params (Item :type "/Game/Blueprints/Data/ItemType Enum" :default "NewEnumerator0") (RequestingSlot :type "/Game/Blueprints/BP_ButtonToggle Object Reference"))
  (returns (CanActivate :type Boolean))
  (return false))

(fn `UserConstructionScript`)