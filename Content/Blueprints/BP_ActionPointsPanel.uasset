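; Action points panel that shows current points out of a maximum as a row of light bulbs.
; SetUpGauge, also called from the construction script, spawns centered, evenly spaced bulb meshes, each with a dynamic emissive material.
; UpdateGauge selects only the bulbs between old and new amounts and fades their emissive through a timeline, storing the new amount when finished.
; ErrorFeedback animates an error parameter across all bulbs; AskForActivation always returns false.
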(event EventErrorFeedback
  (bind _emissivetrack (Timeline|ErrorTimeline PlayFromStart)
    (:Update
      (Rendering|Material|SetScalarParameterValue (Variables|Default|GetLightBulbMaterialArray) "ErrorLerp" _emissivetrack :!class /Script/Engine.MaterialInstanceDynamic))))

(event EventSetUpGauge
  (params (TotalValue :type Integer) (CurrentValue :type Integer))
  (Utilities|Array|Clear (Variables|Default|GetLightBulbMaterialArray))
  (bind _output_get (Variables|Default|SetMaxActionPoints TotalValue))
  (Variables|Default|SetCurrentActionPoints _output_get)
  (for _index (range 0 (- (Variables|Default|GetMaxActionPoints) 1))
    (bind _returnvalue (AddComponent|AddStaticMeshComponent false (Math|Transform|MakeTransform (Math|Vector|MakeVector (|((CurrentIndex*distance)-((round((TotalIndex/2)))*distance)) _index (Variables|Default|GetLightbulbSeparation) (Variables|Default|GetMaxActionPoints)) 0.0 0.0) "0,90.000000, 0" "0.200000,0.200000,0.200000")))
    (Utilities|FlowControl|Sequence
      (:then_0
        (Components|StaticMesh|SetStaticMesh _returnvalue "/Game/Meshes/SM_GaugeGlass.SM_GaugeGlass"))
      (:then_1
        (bind _returnvalue_2 (Rendering|Material|CreateDynamicMaterialInstance _returnvalue 0 "/Game/Materials/MI_GenericEmissive.MI_GenericEmissive" "None" :!class /Script/Engine.PrimitiveComponent))
        (Utilities|Array|Add (Variables|Default|GetLightBulbMaterialArray) _returnvalue_2))))
  (CallFunction|UpdateGauge CurrentValue))

(event EventUpdateGauge
  (params (CurrentAmount :type Integer))
  (bind (_lightbulbstomodify _shouldupdate _currentemissiveness _targetemissiveness) (CallFunction|SelectLightBulbstoChange CurrentAmount))
  (if _shouldupdate
    (bind _lerptrack (Timeline|LightStatusTimeline PlayFromStart)
      (:Update
        (Rendering|Material|SetScalarParameterValue _lightbulbstomodify "Emissive" (Math|Float|Lerp _currentemissiveness _targetemissiveness _lerptrack) :!class /Script/Engine.MaterialInstanceDynamic))
      (:Finished
        (Variables|Default|SetCurrentActionPoints CurrentAmount)))))

(fn ConstructionScript
  (CallFunction|SetUpGauge (Variables|Default|GetMaxActionPoints) (Variables|Default|GetCurrentActionPoints)))

(fn SelectLightBulbstoChange
  (params (NewLightBulbAmount :type Integer))
  (if (!= (Math|Integer|Clamp(Integer) NewLightBulbAmount 0 (Variables|Default|GetMaxActionPoints)) (Variables|Default|GetCurrentActionPoints))
    (bind _output_get (LocalVariables|SetTargetAmount NewLightBulbAmount))
    (if (< _output_get (Variables|Default|GetCurrentActionPoints))
      (for _index (range (LocalVariables|GetTargetAmount) (- (Variables|Default|GetCurrentActionPoints) 1))
        (Utilities|Array|Add (LocalVariables|GetLightBulbMaterialsToModify) (Utilities|Array|Get(acopy) (Variables|Default|GetLightBulbMaterialArray) _index)))
      (return (LocalVariables|GetLightBulbMaterialsToModify) true 15.0 0.0)
      (else
        (for _index_2 (range (Variables|Default|GetCurrentActionPoints) (- (LocalVariables|GetTargetAmount) 1))
          (Utilities|Array|Add (LocalVariables|GetLightBulbMaterialsToModify) (Utilities|Array|Get(acopy) (Variables|Default|GetLightBulbMaterialArray) _index_2)))
        (return (LocalVariables|GetLightBulbMaterialsToModify) true 0.0 15.0)))
    (else
      (return 0 false 0.0 0.0))))

(fn AskforActivation
  (params (Item :type ItemType%20Enum :default "NewEnumerator0") (RequestingSlot :type BP%20Button%20Toggle%20Object%20Reference))
  (return false))