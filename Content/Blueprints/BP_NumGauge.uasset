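; BP_NumGauge is a mechanical-style number gauge that shows a clamped amount on rotating unit and tens dials, 36 degrees per digit.
; Updates enable Actor Tick to spin the unit dial at constant speed, stopping and snapping near the target.
; Tens changes detected from unit rotation play a timeline lerp on the second dial.
; Start and stop calls bracket movement, with CumulatedAmount holding a follow-up value; an older timeline method remains unused.
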(event `self.UpdateGauge`
  (params (CurrentAmount :type Integer))
  (bind (_currentunitrotation_roll _currentunitrotation_pitch) (`KismetMathLibrary.BreakRotator` (`self.CurrentUnitRotation`)))
  (bind (_currentunitrotation_roll_2 _currentunitrotation_pitch_2) (`KismetMathLibrary.BreakRotator` (`self.CurrentUnitRotation`)))
  (bind (_targetunitrotation_roll _targetunitrotation_pitch) (`KismetMathLibrary.BreakRotator` (`self.TargetUnitRotation`)))
  (bind _returnvalue (`KismetMathLibrary.Clamp` CurrentAmount 0 (`self.MaxAmount`)))
  ;[1 1 1] Update Gauge Event
  (if (and (!= _returnvalue (`self.CurrentAmount`)) (not (`TimelineComponent.IsPlaying` (`self.GaugeRotationTimeline`))))
    (bind _output_get (set `self.TargetAmount` _returnvalue))
    (set `self.TargetUnitRotation` (`KismetMathLibrary.MakeRotator` 0.0 (+ (* (- (`self.CurrentAmount`) _output_get) 36.0) _currentunitrotation_pitch)))
    (if (< _currentunitrotation_pitch_2 _targetunitrotation_pitch)
      (set `self.UpdateDirection` 1.0)
      (else
        (set `self.UpdateDirection` -1.0)))
    (`self.SetActorTickEnabled` true)
    (`self.StartedUpdating`)
    (else
      (set `self.CumulatedAmount` _returnvalue))))

(event `self.SetUpGauge`
  (params (TotalValue :type Integer) (CurrentValue :type Integer))
  ;[1 1 1] Set-Up Gauge Event
  (bind _output_get (set `self.MaxAmount` TotalValue))
  (bind _returnvalue (`KismetMathLibrary.Clamp` CurrentValue 0 _output_get))
  (bind _output_get_2 (set `self.CurrentUnitRotation` (`KismetMathLibrary.MakeRotator` 0.0 (* _returnvalue -36.0))))
  (`SceneComponent.K2_SetRelativeRotation` (`self.UnitGauge`) _output_get_2 false false)
  (bind _output_get_3 (set `self.CurrentDecimalRotation` (`KismetMathLibrary.MakeRotator` 0.0 (* (/ _returnvalue 10) -36.0))))
  (`SceneComponent.K2_SetRelativeRotation` (`self.DecimalGauge`) _output_get_3 false false)
  (bind _output_get_4 (set `self.CurrentAmount` _returnvalue))
  (set `self.CurrentDecimals` (/ _output_get_4 10)))

(event `self.ReceiveTick`
  (params (DeltaSeconds :type "Float (single-precision)"))
  (bind (_currentunitrotation_roll _currentunitrotation_pitch) (`KismetMathLibrary.BreakRotator` (`self.CurrentUnitRotation`)))
  (bind _returnvalue (+ (* (* DeltaSeconds (`self.UpdateSpeed`)) (`self.UpdateDirection`)) _currentunitrotation_pitch))
  ;[1 1 1] Update Gauge (Event Tick)
  (bind _output_get (set `self.CurrentUnitRotation` (`KismetMathLibrary.MakeRotator` 0.0 _returnvalue)))
  (`|ExecutionSequence`
    (:`then_0`
      (`SceneComponent.K2_SetRelativeRotation` (`self.UnitGauge`) _output_get false false)
      (if (== _output_get (`self.TargetUnitRotation`) :`ErrorTolerance` 2.5)
        (`self.StopTicking`)))
    (:`then_1`
      (bind _newdecimalrotation (`self.CheckForDecimalChange` _returnvalue)
        (:`ShouldUpdate`
          (set `self.TargetDecimalRotation` _newdecimalrotation)
          (bind (_direction _lerptrack) (`Timeline|DecimalRotationTimeline` :!via `PlayFromStart`)
            (:`Update`
              (`SceneComponent.K2_SetRelativeRotation` (`self.DecimalGauge`) (`KismetMathLibrary.RLerp` (`self.CurrentDecimalRotation`) (`self.TargetDecimalRotation`) _lerptrack) false false))
            (:`Finished`
              (set `self.CurrentDecimalRotation` (`self.TargetDecimalRotation`)))))))))

(event `StopTicking`
  (bind _targetunitrotation (`self.TargetUnitRotation`))
  (bind _targetamount (`self.TargetAmount`))
  ;[1 1 1] Stop Event Tick
  (`self.SetActorTickEnabled` false)
  (`SceneComponent.K2_SetRelativeRotation` (`self.UnitGauge`) _targetunitrotation false false)
  (set `self.CurrentUnitRotation` _targetunitrotation)
  (set `self.CurrentAmount` _targetamount)
  (set `self.CurrentDecimals` (/ _targetamount 10))
  (if (!= (`self.CumulatedAmount`) 0)
    (`self.UpdateGauge` (`self.CumulatedAmount`))
    (set `self.CumulatedAmount` 0)
    (else
      (`self.StoppedUpdating`))))

(fn `AskForActivation`
  (params (Item :type "/Game/Blueprints/Data/ItemType Enum" :default "NewEnumerator0") (RequestingSlot :type "/Game/Blueprints/BP_ButtonToggle Object Reference"))
  (returns (CanActivate :type Boolean))
  (return false))

(fn `CalculateRotation`
  (params (NewAmount :type Integer))
  (returns (NewRotation :type "Float (double-precision)"))
  (bind _returnvalue (- (`self.CurrentAmount`) NewAmount))
  (if (<= NewAmount (`self.CurrentAmount`))
    (return (* _returnvalue 36.0))
    (else
      (return (* _returnvalue 36.0)))))

(fn `UserConstructionScript`)